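; BP_Grabber is a component that lets its owner pick up, carry and release BP_Inspectable actors.
; Grab sphere-traces along the owner's camera forward vector within Range, then attaches a grabbable hit component to the owner's PhysicsHandle at its center of mass.
; UpdateGrabLocation moves the handle target to a supplied root's transform while holding.
; Release drops the component, notifies the inspectable and clears the held state.
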(fn `GetActorInReach`
  (returns (`Return Value` :type "/Game/Blueprints/Actors/BP_Inspectable Object Reference") (`Out Hit Hit Component` :type "PrimitiveComponent Object Reference"))
  (bind _returnvalue (`Actor.GetComponentByClass` (`self.GetOwner`) "/Script/Engine.CameraComponent"))
  (bind _returnvalue_2 (`SceneComponent.K2_GetComponentLocation` _returnvalue))
  (`/Engine/EditorBlueprintResources/StandardMacros.IsValid` _returnvalue
    (:`Is Valid`
      (bind (_outhit _returnvalue_3) (`KismetSystemLibrary.SphereTraceSingle` _returnvalue_2 (+ _returnvalue_2 (* (`SceneComponent.GetForwardVector` _returnvalue) (`self.Range`))) 4.0 "TraceTypeQuery1"))
      (if _returnvalue_3
        (bind _asbp_inspectable (cast `/Game/Blueprints/Actors/BP_Inspectable` (`.HitActor` (`GameplayStatics.BreakHitResult` _outhit)))
          (:`then`
            (return _asbp_inspectable (`.HitComponent` (`GameplayStatics.BreakHitResult` _outhit))))
          (:`CastFailed`
            _)))
      (return null null))
    (:`Is Not Valid`
      (return null null))))

(fn `GetPhysicsHandle`
  (returns (ReturnValue :type "PhysicsHandleComponent Object Reference"))
  (return (`Actor.GetComponentByClass` (`self.GetOwner`) "/Script/Engine.PhysicsHandleComponent")))

(fn `Grab`
  (params (GrabLocation :type "SceneComponent Object Reference"))
  (bind (_return_value _out_hit_hit_component) (`self.GetActorInReach`))
  (`/Engine/EditorBlueprintResources/StandardMacros.IsValid` _return_value
    (:`Is Valid`
      (if (`/Game/Blueprints/Actors/BP_Inspectable.CanBeGrabbed` _return_value)
        (`/Game/Blueprints/Actors/BP_Inspectable.Grab` _return_value)
        (`PhysicsHandleComponent.GrabComponentAtLocationWithRotation` :`self` (`self.GetPhysicsHandle`) :`Component` _out_hit_hit_component :`Location` (`PrimitiveComponent.GetCenterOfMass` _out_hit_hit_component "None"))
        (set `self.HeldObject` _return_value)
        (set `self.IsHolding` true)))))

(fn `Release`
  (bind _heldobject (`self.HeldObject`))
  (`/Engine/EditorBlueprintResources/StandardMacros.IsValid` _heldobject
    (:`Is Valid`
      (`PhysicsHandleComponent.ReleaseComponent` (`self.GetPhysicsHandle`))
      (`/Game/Blueprints/Actors/BP_Inspectable.Release` _heldobject)
      (set `self.HeldObject` null)
      (set `self.IsHolding` false))))

(fn `UpdateGrabLocation`
  (params (`Grab Root` :type "SceneComponent Object Reference"))
  (if (`self.IsHolding`)
    (`PhysicsHandleComponent.SetTargetLocationAndRotation` (`self.GetPhysicsHandle`) (`SceneComponent.K2_GetComponentLocation` `Grab Root`) (`SceneComponent.K2_GetComponentRotation` `Grab Root`))))