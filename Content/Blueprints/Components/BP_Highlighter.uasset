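; BP_Highlighter is a component that detects which highlightable actor the camera is looking at.
; FindHighlight runs a thin sphere trace along the camera's forward vector up to Range, keeping only hit actors that implement BPI_Highlight.
; When the focused actor changes, it sends begin and end focus interface messages to the new and previous actors.
; The event graph is empty, so the component does not run the check itself.
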(event `self.ReceiveTick`
  (params (DeltaSeconds :type "Float (single-precision)")))

(fn `FindHighlight`
  (bind _camera (`self.Camera`))
  (bind _focusedactor (`self.FocusedActor`))
  (bind _previousfocusedactor (`self.PreviousFocusedActor`))
  (bind _returnvalue (`SceneComponent.K2_GetComponentLocation` _camera))
  (`/Engine/EditorBlueprintResources/StandardMacros.IsValid` _camera
    (:`Is Valid`
      (bind (_outhit _returnvalue_2) (`KismetSystemLibrary.SphereTraceSingle` _returnvalue (+ _returnvalue (* (`SceneComponent.GetForwardVector` _camera) (`self.Range`))) 4.0 "TraceTypeQuery1"))
      (set `self.PreviousFocusedActor` (`self.FocusedActor`))
      (if _returnvalue_2
        (bind (_bblockinghit _binitialoverlap _time _distance _location _impactpoint _normal _impactnormal _physmat _hitactor) (`GameplayStatics.BreakHitResult` _outhit))
        (if (`KismetSystemLibrary.DoesImplementInterface` _hitactor "/Game/Blueprints/Interfaces/BPI_Highlight.BPI_Highlight_C")
          (set `self.FocusedActor` _hitactor)
          (else
            (set `self.FocusedActor` null :!label _label)))
        (else
          (goto _label)))
      (if (!= (`self.FocusedActor`) (`self.PreviousFocusedActor`))
        (`|ExecutionSequence`
          (:`then_0`
            (`/Engine/EditorBlueprintResources/StandardMacros.IsValid` _focusedactor
              (:`Is Valid`
                (message `/Game/Blueprints/Interfaces/BPI_Highlight.Begin Focus` _focusedactor))))
          (:`then_1`
            (`/Engine/EditorBlueprintResources/StandardMacros.IsValid` _previousfocusedactor
              (:`Is Valid`
                (message `/Game/Blueprints/Interfaces/BPI_Highlight.End Focus` _previousfocusedactor)))))))))