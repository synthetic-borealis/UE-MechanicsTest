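; Inspectable prop actor that can be grabbed, released and highlighted on focus through a custom depth stencil.
; Grabbing enables mesh physics and disables shadow casting; releasing within ReturnDistance plays a timeline that lerps it back to the transform cached at construction.
; Released farther away, it stays simulated until a hit plus a short trace along its down vector freezes it after a brief delay.
; GetFinalTransform exposes an optional override of the original transform.
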(event `Grab`
  (if (and (`self.CanBeGrabbed`) (`self.GrabEnabled`))
    (`PrimitiveComponent.SetSimulatePhysics` (`self.StaticMesh`) true)
    (set `self.CanBeGrabbed` false)
    (`PrimitiveComponent.SetCastShadow` (`self.StaticMesh`) false)))

(event `Release`
  (`PrimitiveComponent.SetCastShadow` (`self.StaticMesh`) true)
  (if (<= (`KismetMathLibrary.Vector_Distance` (`self.OriginalLocation`) (`self.K2_GetActorLocation`)) (`self.Return Distance`))
    (`PrimitiveComponent.SetSimulatePhysics` (`self.StaticMesh`) false)
    (bind (_direction _alpha) (`Timeline|ReturnToPlace`)
      (:`Update`
        (`|ExecutionSequence`
          (:`then_0`
            (`self.RestoreLocation` _alpha))
          (:`then_1`
            (`self.RestoreRotation` _alpha))))
      (:`Finished`
        (`PrimitiveComponent.SetSimulatePhysics` (`self.StaticMesh`) false)
        (set `self.CanBeGrabbed` true)))
    (else
      (set `self.CanBeGrabbed` true)
      (set `self.HasHitGround` false))))

(event `self.StaticMesh.OnComponentHit`
  (params (HitComponent :type "PrimitiveComponent Object Reference") (OtherActor :type "Actor Object Reference") (OtherComp :type "PrimitiveComponent Object Reference") (NormalImpulse :type "Vector Structure") (Hit :type "HitResult Structure (by ref)"))
  (bind _returnvalue (`self.K2_GetActorLocation`))
  (if (not (`self.HasHitGround`))
    (bind (_outhit _returnvalue_2) (`KismetSystemLibrary.LineTraceSingle` _returnvalue (- _returnvalue (`self.GetActorUpVector`)) "TraceTypeQuery1"))
    (if _returnvalue_2
      (`KismetSystemLibrary.Delay` 0.2)
      (`PrimitiveComponent.SetSimulatePhysics` (`self.StaticMesh`) false)
      (set `self.HasHitGround` true))))

(event `/Game/Blueprints/Interfaces/BPI_Highlight.Begin Focus`
  (if (`self.Higlight Enabled?`)
    (`PrimitiveComponent.SetCustomDepthStencilValue` (`self.StaticMesh`) 2)))

(event `/Game/Blueprints/Interfaces/BPI_Highlight.End Focus`
  (`PrimitiveComponent.SetCustomDepthStencilValue` (`self.StaticMesh`) 0))

(event `/Game/Blueprints/Interfaces/BPI_Highlight.SetHighlightEnabled`
  (params (Enabled :type Boolean))
  (set `self.Higlight Enabled?` Enabled))

(fn `GetFinalTransform`
  (returns (`Return Value` :type "Transform Structure"))
  (if (`self.HasFinalTransform`)
    (return (`self.FinalTransform`))
    (else
      (return (`KismetMathLibrary.MakeTransform` (`self.OriginalLocation`) (`self.OriginalRotation`))))))

(fn `GetHighlightEnabled`
  (returns (`Return Value` :type Boolean))
  (return (`self.Higlight Enabled?`)))

(fn `RestoreLocation`
  (params (Alpha :type "Float (double-precision)"))
  (`self.K2_SetActorLocation` (`KismetMathLibrary.VLerp` (`self.K2_GetActorLocation`) (`self.OriginalLocation`) Alpha)))

(fn `RestoreRotation`
  (params (Alpha :type "Float (double-precision)"))
  (`self.K2_SetActorRotation` (`KismetMathLibrary.RLerp` (`self.K2_GetActorRotation`) (`self.OriginalRotation`) Alpha)))

(fn `UserConstructionScript`
  (`SceneComponent.SetMobility` (`self.StaticMesh`) "Movable")
  (set `self.OriginalLocation` (`self.K2_GetActorLocation`))
  (set `self.OriginalRotation` (`self.K2_GetActorRotation`))
  (`PrimitiveComponent.SetRenderCustomDepth` (`self.StaticMesh`) true))